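; BP_Item_Attach2 is an attach point that holds a BP_Item2 of a configured class for one maneuver index.
; BeginPlay spawns that item snapped to itself, enabling interaction and showing its mesh only if the player pawn's Index matches.
; While interactable and empty, it snaps overlapping items of that exact class onto itself.
; InvertHidden selects whether attaching or detaching hides the mesh and ends interaction.
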(event `self.ReceiveBeginPlay`
  (bind _asbp_pawn (cast `/Game/BP_Character/BP_Pawn` (`GameplayStatics.GetPlayerPawn` 0)))
  (set `self.BP_Pawn` _asbp_pawn)
  (`self.CAN INTERACT`)
  (bind _returnvalue (`|SpawnActorFromClass` (`self.BP_Item_To_Attach`) (`self.GetTransform`) "Undefined" "OverrideRootScale" null true (`self.Maneuver_index`) null))
  (`self.K2_AttachToActor` _returnvalue self "None" "SnapToTarget" "SnapToTarget" "KeepWorld" true))

(event `CAN INTERACT`
  (bind _output_get (set `self.Can_Interact?` (== (`/Game/BP_Character/BP_Pawn.index` (`self.BP_Pawn`)) (`self.Maneuver_index`))))
  (`self.HIDE / SHOW MESH` (not _output_get)))

(event `self.StaticMeshComponent.OnComponentBeginOverlap`
  (params (OverlappedComponent :type "PrimitiveComponent Object Reference") (OtherActor :type "Actor Object Reference") (OtherComp :type "PrimitiveComponent Object Reference") (OtherBodyIndex :type Integer) (bFromSweep :type Boolean) (SweepResult :type "HitResult Structure (by ref)"))
  (if (`self.Can_Interact?`)
    (if (not (`self.Has_Attached_BP_Item?`))
      (bind _asbp_item_2 (cast `/Game/BP_Items/NOJALANALB/BP_Item2` OtherActor))
      (if (== (`GameplayStatics.GetObjectClass` _asbp_item_2) (`self.BP_Item_To_Attach`))
        (set `self.Has_Attached_BP_Item?` true)
        (set `/Game/BP_Items/NOJALANALB/BP_Item2.BP_Item_Attach` self _asbp_item_2)
        (`self.K2_AttachToActor` _asbp_item_2 self "None" "SnapToTarget" "SnapToTarget" "KeepWorld" true)
        (if (`self.Invert_Hidden`)
          (set `/Game/BP_Items/NOJALANALB/BP_Item2.Can_Interact?` false _asbp_item_2)
          (set `self.Can_Interact?` false)
          (`self.HIDE / SHOW MESH` (`self.Invert_Hidden`)))))))

(event `DettachEvt`
  (if (`self.Can_Interact?`)
    (set `self.Has_Attached_BP_Item?` false)
    (if (not (`self.Invert_Hidden`))
      (set `self.Can_Interact?` false))
    (`self.HIDE / SHOW MESH` (not (`self.Invert_Hidden`)))))

(event `HIDE / SHOW MESH`
  (params (hide :type Boolean))
  (`SceneComponent.SetHiddenInGame` (`self.StaticMeshComponent`) hide false))

(fn `UserConstructionScript`)