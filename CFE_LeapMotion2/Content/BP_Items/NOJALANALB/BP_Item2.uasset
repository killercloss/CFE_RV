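; BP_Item2 is an item actor that a player can pick up and drop when their pawn's index matches the item's index.
; The CANINTERACT event, run at BeginPlay, caches that match against the first player's BP_Pawn.
; Pickup attaches it to the hand's ObjectSocket, keeping world transform, and notifies any valid BPItemAttach to detach.
; Drop detaches it in place; both actions turn mesh physics simulation off.
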(event `CAN INTERACT`
  (set `self.Can_Interact?` (== (`/Game/BP_Character/BP_Pawn.index` (`self.BP_Pawn`)) (`self.Item_Index`))))

(event `self.ReceiveBeginPlay`
  (bind _asbp_pawn (cast `/Game/BP_Character/BP_Pawn` (`GameplayStatics.GetPlayerPawn` 0)))
  (set `self.BP_Pawn` _asbp_pawn)
  (`self.CAN INTERACT`))

(event `/Game/BP_Items/BP_ItemInterface.ItemPickUp`
  (params (HandToAttach :type "SkeletalMeshComponent Object Reference"))
  (if (`self.Can_Interact?`)
    (`PrimitiveComponent.SetSimulatePhysics` (`self.StaticMeshComponent`) false)
    (`self.K2_AttachToComponent` self HandToAttach "ObjectSocket" "KeepWorld" "KeepWorld" "KeepWorld" true)
    (bind _bp_item_attach (`self.BP_Item_Attach`)
      (:`then`
        (`/Game/BP_Items/NOJALANALB/BP_Item_Attach2.DettachEvt` _bp_item_attach))
      (:`else`))))

(event `/Game/BP_Items/BP_ItemInterface.ItemDrop`
  (if (`self.Can_Interact?`)
    (`PrimitiveComponent.SetSimulatePhysics` (`self.StaticMeshComponent`) false)
    (`self.K2_DetachFromActor` self "KeepWorld" "KeepWorld" "KeepWorld")))

(fn `UserConstructionScript`)