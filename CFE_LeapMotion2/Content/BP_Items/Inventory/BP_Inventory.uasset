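; BP_Inventory is a Leap Motion inventory that presents one item at a time from a list.
; It spawns the current entry's actor on a sphere, passing that entry's interaction and process settings plus itself.
; Grabbing hands overlapping Next or Back cycle items, while Cubeta toggles item and button visibility and collision.
; A detach event decrements quantity or removes depleted entries, respawning after decrements or when removal pushes the index out of range.
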(event `self.ReceiveBeginPlay`
  (`self.SPAWN_ITEM`))

(event `SPAWN_ITEM`
  (bind _sphere (`self.Sphere`))
  (bind (_output_bp_item_class _output_quantity _output_can_interact_ _output_is_not_trigger_ _output_process_index _output_functionality _output_inverted _output_process_index_change _output_set_inverted_to) (break `/Game/BP_Items/Inventory/BP_Item_Structure` (`|GetArrayItem` (`self.Inventory_List`) (`self.index`))))
  (bind _returnvalue (`|SpawnActorFromClass` _output_bp_item_class (`SceneComponent.K2_GetComponentToWorld` _sphere) "Undefined" "OverrideRootScale" null _output_can_interact_ _output_is_not_trigger_ self _output_process_index _output_functionality _output_inverted _output_process_index_change _output_set_inverted_to null))
  (bind _output_get (set `self.BP_Item` _returnvalue))
  (`self.K2_AttachToComponent` _output_get _sphere "None" "SnapToTarget" "SnapToTarget" "KeepWorld" true))

(event `self.Next.OnComponentBeginOverlap`
  (params (OverlappedComponent :type "PrimitiveComponent Object Reference") (OtherActor :type "Actor Object Reference") (OtherComp :type "PrimitiveComponent Object Reference") (OtherBodyIndex :type Integer) (bFromSweep :type Boolean) (SweepResult :type "HitResult Structure (by ref)"))
  (bind _returnvalue (+ (`self.index`) 1))
  (bind _asleap_desktop_low_poly (cast `/LeapMotion/DirectRigging/LowPoly/LeapDesktopLowPoly` OtherActor))
  (if (or (`/LeapMotion/DirectRigging/LowPoly/LeapDesktopLowPoly.leftGrab` _asleap_desktop_low_poly) (`/LeapMotion/DirectRigging/LowPoly/LeapDesktopLowPoly.rightGrab` _asleap_desktop_low_poly))
    (if (< _returnvalue (`KismetArrayLibrary.Array_Length` (`self.Inventory_List`)))
      (set `self.index` _returnvalue)
      (bind _bp_item (`self.BP_Item`)
        (:`then`
          (`self.K2_DestroyActor` _bp_item)
          (set `self.BP_Item` null))
        (:`else`
          _))
      (`self.SPAWN_ITEM`))))

(event `self.Back.OnComponentBeginOverlap`
  (params (OverlappedComponent :type "PrimitiveComponent Object Reference") (OtherActor :type "Actor Object Reference") (OtherComp :type "PrimitiveComponent Object Reference") (OtherBodyIndex :type Integer) (bFromSweep :type Boolean) (SweepResult :type "HitResult Structure (by ref)"))
  (bind _returnvalue (- (`self.index`) 1))
  (bind _asleap_desktop_low_poly (cast `/LeapMotion/DirectRigging/LowPoly/LeapDesktopLowPoly` OtherActor))
  (if (or (`/LeapMotion/DirectRigging/LowPoly/LeapDesktopLowPoly.leftGrab` _asleap_desktop_low_poly) (`/LeapMotion/DirectRigging/LowPoly/LeapDesktopLowPoly.rightGrab` _asleap_desktop_low_poly))
    (if (>= _returnvalue 0)
      (set `self.index` _returnvalue)
      (bind _bp_item (`self.BP_Item`)
        (:`then`
          (`self.K2_DestroyActor` _bp_item)
          (set `self.BP_Item` null))
        (:`else`
          _))
      (`self.SPAWN_ITEM`))))

(event `DETTACH_EVENT`
  (bind _inventory_list (`self.Inventory_List`))
  (bind _index (`self.index`))
  (bind _returnvalue (`KismetArrayLibrary.Array_Length` _inventory_list))
  (bind (_output_bp_item_class _output_quantity _output_can_interact_ _output_is_not_trigger_ _output_process_index _output_functionality _output_inverted _output_process_index_change _output_set_inverted_to) (break `/Game/BP_Items/Inventory/BP_Item_Structure` (`|GetArrayItem` (`self.Inventory_List`) (`self.index`))))
  (bind _returnvalue_2 (- _output_quantity 1))
  (if (<= _returnvalue_2 0)
    (`KismetArrayLibrary.Array_Remove` _inventory_list _index)
    (if (>= _index _returnvalue)
      (set `self.index` (- _returnvalue 1))
      (`self.SPAWN_ITEM` :!label _label))
    (else
      (`KismetArrayLibrary.Array_Set` (`self.Inventory_List`) (`self.index`) (make `/Game/BP_Items/Inventory/BP_Item_Structure` _output_bp_item_class _returnvalue_2 _output_can_interact_ _output_is_not_trigger_ _output_process_index _output_functionality _output_inverted _output_process_index_change _output_set_inverted_to))
      (goto _label))))

(event `self.Cubeta.OnComponentBeginOverlap`
  (params (OverlappedComponent :type "PrimitiveComponent Object Reference") (OtherActor :type "Actor Object Reference") (OtherComp :type "PrimitiveComponent Object Reference") (OtherBodyIndex :type Integer) (bFromSweep :type Boolean) (SweepResult :type "HitResult Structure (by ref)"))
  (bind _asleap_desktop_low_poly (cast `/LeapMotion/DirectRigging/LowPoly/LeapDesktopLowPoly` OtherActor))
  (if (or (`/LeapMotion/DirectRigging/LowPoly/LeapDesktopLowPoly.leftGrab` _asleap_desktop_low_poly) (`/LeapMotion/DirectRigging/LowPoly/LeapDesktopLowPoly.rightGrab` _asleap_desktop_low_poly))
    (bind _output_get (set `self.hide&showInventory` (not (`self.hide&showInventory`))))
    (if _output_get
      (`self.SHOW_INVENTORY`)
      (else
        (`self.HIDE_INVENTORY`)))))

(event `HIDE_INVENTORY`
  (bind _back (`self.Back`))
  (bind _next (`self.Next`))
  (`|ExecutionSequence`
    (:`then_0`
      (bind _bp_item (`self.BP_Item`)
        (:`then`
          (bind _staticmeshcomponent (`StaticMeshActor.StaticMeshComponent` _bp_item))
          (`SceneComponent.SetVisibility` _staticmeshcomponent false false)
          (`PrimitiveComponent.SetCollisionEnabled` _staticmeshcomponent "NoCollision"))
        (:`else`)))
    (:`then_1`
      (`SceneComponent.SetVisibility` _back false false)
      (`PrimitiveComponent.SetCollisionEnabled` _back "NoCollision"))
    (:`then_2`
      (`SceneComponent.SetVisibility` _next false false)
      (`PrimitiveComponent.SetCollisionEnabled` _next "NoCollision"))))

(event `SHOW_INVENTORY`
  (bind _back (`self.Back`))
  (bind _next (`self.Next`))
  (`|ExecutionSequence`
    (:`then_0`
      (bind _bp_item (`self.BP_Item`)
        (:`then`
          (bind _staticmeshcomponent (`StaticMeshActor.StaticMeshComponent` _bp_item))
          (`SceneComponent.SetVisibility` _staticmeshcomponent true false)
          (`PrimitiveComponent.SetCollisionEnabled` _staticmeshcomponent "QueryAndPhysics"))
        (:`else`)))
    (:`then_1`
      (`SceneComponent.SetVisibility` _back true false)
      (`PrimitiveComponent.SetCollisionEnabled` _back "QueryAndPhysics"))
    (:`then_2`
      (`SceneComponent.SetVisibility` _next true false)
      (`PrimitiveComponent.SetCollisionEnabled` _next "QueryAndPhysics"))))

(fn `UserConstructionScript`)