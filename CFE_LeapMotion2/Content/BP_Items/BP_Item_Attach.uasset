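; BP_Item_Attach is an attach point that snaps an item of a specified BP_Item class onto itself.
; When its mesh overlaps a matching item while empty, it gives the item a back-reference, attaches it with world scale kept and marks itself occupied.
; DetachEvt clears the occupied flag but performs no detachment itself.
; Both events toggle the point's mesh visibility, with InvertHidden setting the polarity.
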(event `self.ReceiveBeginPlay`
  (bind _asbp_pawn (cast `/Game/BP_Character/BP_Pawn` (`GameplayStatics.GetPlayerPawn` 0)))
  (set `self.BP_Pawn` _asbp_pawn))

(event `self.StaticMeshComponent.OnComponentBeginOverlap`
  (params (OverlappedComponent :type "PrimitiveComponent Object Reference") (OtherActor :type "Actor Object Reference") (OtherComp :type "PrimitiveComponent Object Reference") (OtherBodyIndex :type Integer) (bFromSweep :type Boolean) (SweepResult :type "HitResult Structure (by ref)"))
  (if (not (`self.Has_Attached_BP_Item?`))
    (bind _asbp_item (cast `/Game/BP_Items/BP_Item` OtherActor))
    (if (== (`GameplayStatics.GetObjectClass` _asbp_item) (`self.BP_Item_To_Attach`))
      (set `self.Has_Attached_BP_Item?` true)
      (set `/Game/BP_Items/BP_Item.BP_Item_Attach` self _asbp_item)
      (`self.K2_AttachToActor` _asbp_item self "None" "SnapToTarget" "SnapToTarget" "KeepWorld" true)
      (`self.HIDE / SHOW MESH` (`self.Invert_Hidden`)))))

(event `DettachEvt`
  (set `self.Has_Attached_BP_Item?` false)
  (`self.HIDE / SHOW MESH` (not (`self.Invert_Hidden`))))

(event `HIDE / SHOW MESH`
  (params (hide :type Boolean))
  (`SceneComponent.SetHiddenInGame` (`self.StaticMeshComponent`) hide false))

(fn `UserConstructionScript`)