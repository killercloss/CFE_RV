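; BP_Pertiga is a pickup item that can be attached to and released from a hand.
; ItemPickUp prints a debug string, snaps the item to the hand's ObjectSocket while keeping world rotation, then disables mesh physics.
; ItemDrop detaches it at its world transform but also leaves physics disabled, so it does not fall.
; An unconnected chain for class-filtered BP_Item attachment with an occupied flag never runs.
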(event `self.ReceiveBeginPlay`)

(event `/Game/BP_Items/BP_ItemInterface.ItemPickUp`
  (params (HandToAttach :type "SkeletalMeshComponent Object Reference"))
  ;[1 1 1] ATTACH & DETTACH OBJECT
  (`KismetSystemLibrary.PrintString` "Hello")
  (`self.K2_AttachToComponent` self HandToAttach "ObjectSocket" "SnapToTarget" "KeepWorld" "KeepWorld" true)
  (`PrimitiveComponent.SetSimulatePhysics` (`self.StaticMeshComponent`) false))

(event `/Game/BP_Items/BP_ItemInterface.ItemDrop`
  ;[1 1 1] ATTACH & DETTACH OBJECT
  (`PrimitiveComponent.SetSimulatePhysics` (`self.StaticMeshComponent`) false)
  (`self.K2_DetachFromActor` self "KeepWorld" "KeepWorld" "KeepWorld"))

(fn `UserConstructionScript`)