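; BP_Item is a base for items that act as either pickable parts or trigger slots in a pawn-tracked, step-based process.
; Slots snap-attach same-class items: non-functional ones at BeginPlay, functional ones on overlap, which then triggers the pawn's process check.
; Pickup attaches parts to a hand socket, frees their slot or inventory, and destroys detached faulty parts.
; The pawn's Index gates interaction and slot visibility, and can alter functionality or inversion.
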(event `self.ReceiveBeginPlay`
  ;[1 1 1] GET THE PAWN
  (bind _asbp_pawn (cast `/Game/BP_Character/BP_Pawn` (`GameplayStatics.GetPlayerPawn` 0)))
  (set `self.BP_Pawn` _asbp_pawn)
  ;[1 1 1] SET THE CLASS TO MATCH
  (set `self.Item_Class_Match` (`GameplayStatics.GetObjectClass` self))
  (`self.CAN_INTERACT_EVENT`)
  ;[1 1 1] CHECK OVERLAPPING ACTORS AT THE BEGINING OF THE GAME
  ;;[1 1 1] GET OVERLAPPING ACTORS
  (if (`KismetMathLibrary.BooleanNOR` (`self.Its_Not_Trigger?`) (`self.Its_Occupied?`))
    (for _array_element (`self.GetOverlappingActors` "BP_Item_C")
      ;;[1 1 1] IF CLASS MATCH & FUNCTIONALITY IS EQUAL TO FALSE
      (bind _asbp_item (cast `/Game/BP_Items/BLUEPRINTS/BP_Item` _array_element))
      (if (== (`GameplayStatics.GetObjectClass` _asbp_item) (`self.Item_Class_Match`))
        (if (not (`/Game/BP_Items/BLUEPRINTS/BP_Item.Functionality` _asbp_item))
          ;;[1 1 1] ATTACH THE BP_ITEM
          (set `/Game/BP_Items/BLUEPRINTS/BP_Item.BP_Item_Attach` self _asbp_item)
          (`self.K2_AttachToActor` _asbp_item self "None" "SnapToTarget" "SnapToTarget" "KeepWorld" true)
          (set `self.Its_Occupied?` true)
          (break))))))

(event `self.StaticMeshComponent.OnComponentBeginOverlap`
  (params (OverlappedComponent :type "PrimitiveComponent Object Reference") (OtherActor :type "Actor Object Reference") (OtherComp :type "PrimitiveComponent Object Reference") (OtherBodyIndex :type Integer) (bFromSweep :type Boolean) (SweepResult :type "HitResult Structure (by ref)"))
  (`self.BP_Inventory`
    (:`then`)
    (:`else`
      (if (`self.Can_Interact?`)
        ;[1 1 1] IF NOT OCCUPIED & CLASS MATCH
        (if (`KismetMathLibrary.BooleanNOR` (`self.Its_Not_Trigger?`) (`self.Its_Occupied?`))
          (bind _asbp_item (cast `/Game/BP_Items/BLUEPRINTS/BP_Item` OtherActor))
          (if (== (`GameplayStatics.GetObjectClass` _asbp_item) (`self.Item_Class_Match`))
            ;[1 1 1] CHECK IF THE COMPONENT WE WANT TO ATTACH WORKS
            (if (`/Game/BP_Items/BLUEPRINTS/BP_Item.Functionality` _asbp_item)
              (set `self.Its_Occupied?` true)
              (set `/Game/BP_Items/BLUEPRINTS/BP_Item.Can_Interact?` false _asbp_item)
              ;[1 1 1] ATTACH THE BP_ITEM
              (set `/Game/BP_Items/BLUEPRINTS/BP_Item.BP_Item_Attach` self _asbp_item)
              (`self.K2_AttachToActor` _asbp_item self "None" "SnapToTarget" "SnapToTarget" "KeepWorld" true)
              (`SceneComponent.SetHiddenInGame` (`self.StaticMeshComponent`) true false)
              (set `self.Working` true)
              (`/Game/BP_Character/BP_Pawn.CHECK_PROCCESS` (`self.BP_Pawn`)))))))))

(event `/Game/BP_Items/BP_ItemInterface.ItemPickUp`
  (params (HandToAttach :type "SkeletalMeshComponent Object Reference"))
  ;[1 1 1] ATTACH & DETTACH OBJECT
  (if (and (`self.Can_Interact?`) (`self.Its_Not_Trigger?`))
    (`self.K2_AttachToComponent` self HandToAttach "ObjectSocket" "KeepWorld" "KeepWorld" "KeepWorld" true)
    (`PrimitiveComponent.SetSimulatePhysics` (`self.StaticMeshComponent`) false)
    (`|ExecutionSequence`
      (:`then_0`
        (bind _bp_item_attach (`self.BP_Item_Attach`)
          (:`then`
            (`self.DETTACH_EVENT` _bp_item_attach)
            (set `self.BP_Item_Attach` null)
            (if (not (`self.Functionality`))
              (`self.K2_DestroyActor`)))
          (:`else`)))
      (:`then_1`
        (bind _bp_inventory (`self.BP_Inventory`)
          (:`then`
            (`/Game/BP_Items/Inventory/BP_Inventory.DETTACH_EVENT` _bp_inventory)
            (set `self.BP_Inventory` null))
          (:`else`))))))

(event `DETTACH_EVENT`
  (bind _inverted (`self.Inverted`))
  (if (not (`self.Its_Not_Trigger?`))
    (`SceneComponent.SetHiddenInGame` (`self.StaticMeshComponent`) _inverted false)
    (set `self.Its_Occupied?` false)
    (set `self.Working` _inverted)
    (`/Game/BP_Character/BP_Pawn.CHECK_PROCCESS` (`self.BP_Pawn`))))

(event `/Game/BP_Items/BP_ItemInterface.ItemDrop`
  ;[1 1 1] ATTACH & DETTACH OBJECT
  (if (and (`self.Can_Interact?`) (`self.Its_Not_Trigger?`))
    (`PrimitiveComponent.SetSimulatePhysics` (`self.StaticMeshComponent`) false)
    (`self.BP_Item_Attach`
      (:`then`)
      (:`else`
        (`self.K2_DetachFromActor` self "KeepWorld" "KeepWorld" "KeepWorld")))))

(event `CAN_INTERACT_EVENT`
  ;[1 1 1] CAN INTERACT?
  (`self.CHANGE_INDEX_EVENT`)
  (bind _bp_pawn (`self.BP_Pawn`)
    (:`then`
      (bind _output_get (set `self.Can_Interact?` (== (`/Game/BP_Character/BP_Pawn.index` _bp_pawn) (`self.Process_Index`))))
      (if _output_get
        (if (not (`self.Its_Not_Trigger?`))
          (`SceneComponent.SetHiddenInGame` (`self.StaticMeshComponent`) false false))
        (elif (not (`self.Its_Not_Trigger?`))
          (`SceneComponent.SetHiddenInGame` (`self.StaticMeshComponent`) true false))))
    (:`else`)))

(event `CHANGE_INDEX_EVENT`
  (bind _process_index_change (`self.Process_Index_Change`))
  (bind _index (`/Game/BP_Character/BP_Pawn.index` (`self.BP_Pawn`)))
  ;[1 1 1] CHANGE INDEX PROCESS
  (if (> _process_index_change 0)
    (if (== _process_index_change _index)
      (set `self.Process_Index` _index)
      (if (`self.Its_Not_Trigger?`)
        (if (`self.Functionality`)
          (set `self.Functionality` (not (`self.Set_Inverted_To`))))
        (else
          (set `self.Inverted` (`self.Set_Inverted_To`))
          (set `self.Working` false))))))

(fn `UserConstructionScript`)