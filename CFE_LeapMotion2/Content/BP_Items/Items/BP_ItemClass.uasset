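; Base item Blueprint for pickable parts that snap together in an index-staged process, acting as items or trigger slots.
; Overlapping a same-class functional item snaps it on, hides the receiving mesh and flags it as working.
; Pickup releases item or tool links and can destroy non-functional items, while begin play links pre-overlapping triggers.
; BP_Pawn's index gates interaction and trigger visibility, can invert state, and attach or detach prompts its process check.
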(event `self.ReceiveBeginPlay`
  (bind _asbp_pawn (cast `/Game/BP_Character/BP_Pawn` (`GameplayStatics.GetPlayerPawn` 0)))
  (set `self.bpPawn` _asbp_pawn)
  (`self.CAN_INTERACT_EVENT`)
  (`self.CHECK_INITIALIZE_EVENT`))

(event `/Game/BP_Items/BP_ItemInterface.ItemPickUp`
  (params (HandToAttach :type "SkeletalMeshComponent Object Reference"))
  ;[1 1 1] PICK UP
  (`self.K2_AttachToComponent` self HandToAttach "ObjectSocket" "KeepWorld" "KeepWorld" "KeepWorld" true)
  (`|ExecutionSequence`
    (:`then_0`
      (bind _bpitemclass (`self.bpItemClass`)
        (:`then`
          (`self.DETTACH_EVENT` _bpitemclass)
          (set `self.bpItemClass` null))
        (:`else`)))
    (:`then_1`
      (bind _bptoolclass (`self.bpToolClass`)
        (:`then`
          (`/Game/BP_Items/Items/BP_Pertigo.DETTACH_EVENT` _bptoolclass)
          (set `self.bpToolClass` null))
        (:`else`))))
  (if (not (`self.functionality`))
    (`self.K2_DestroyActor`)))

(event `CHECK_INITIALIZE_EVENT`
  ;[1 1 1] CHECK IF INITIALIZED
  (for _array_element (`self.GetOverlappingActors` (`GameplayStatics.GetObjectClass` self))
    (bind _asbp_item_class (cast `/Game/BP_Items/Items/BP_ItemClass` _array_element))
    (if (and (`/Game/BP_Items/Items/BP_ItemClass.itsTrigger?` _asbp_item_class) (not (`/Game/BP_Items/Items/BP_ItemClass.functionality` _asbp_item_class)))
      (set `/Game/BP_Items/Items/BP_ItemClass.bpItemClass` self _asbp_item_class)
      (`self.K2_AttachToComponent` _asbp_item_class (`self.StaticMeshComponent`) "None" "SnapToTarget" "SnapToTarget" "KeepWorld" true)
      (set `self.itsOccupied?` true)
      (break))))

(event `/Game/BP_Items/BP_ItemInterface.ItemDrop`
  ;[1 1 1] DROP
  (`SceneComponent.K2_DetachFromComponent` (`self.StaticMeshComponent`) "KeepWorld" "KeepWorld" "KeepWorld" true)
  (`self.bpItemClass`
    (:`then`)
    (:`else`
      (`self.K2_DetachFromActor` self "KeepWorld" "KeepWorld" "KeepWorld"))))

(event `self.StaticMeshComponent.OnComponentBeginOverlap`
  (params (OverlappedComponent :type "PrimitiveComponent Object Reference") (OtherActor :type "Actor Object Reference") (OtherComp :type "PrimitiveComponent Object Reference") (OtherBodyIndex :type Integer) (bFromSweep :type Boolean) (SweepResult :type "HitResult Structure (by ref)"))
  ;[1 1 1] ATTACH
  (if (and (`self.itsTrigger?`) (`self.itsOccupied?`))
    _
    (elif (== (`GameplayStatics.GetObjectClass` OtherActor) (`GameplayStatics.GetObjectClass` self))
      (bind _asbp_item_class (cast `/Game/BP_Items/Items/BP_ItemClass` OtherActor))
      (if (`/Game/BP_Items/Items/BP_ItemClass.functionality` _asbp_item_class)
        (set `self.itsOccupied?` true)
        (set `self.CanInteract?` false)
        (set `/Game/BP_Items/Items/BP_Base.CanInteract?` false _asbp_item_class)
        (set `/Game/BP_Items/Items/BP_ItemClass.bpItemClass` self _asbp_item_class)
        (`self.K2_AttachToActor` _asbp_item_class self "None" "SnapToTarget" "SnapToTarget" "KeepWorld" true)
        (`SceneComponent.SetHiddenInGame` (`self.StaticMeshComponent`) true false)
        (set `self.isWorking?` true)
        (bind _bptoolclass (`self.bpToolClass`)
          (:`then`
            (`/Game/BP_Items/Items/BP_Pertigo.DETTACH_EVENT` _bptoolclass)
            (set `self.bpToolClass` null))
          (:`else`
            _))
        (`/Game/BP_Character/BP_Pawn.CHECK_PROCCESS_EVENT` (`self.bpPawn`))))))

(event `DETTACH_EVENT`
  (bind _inverted (`self.inverted`))
  ;[1 1 1] DETTACH
  (if (not (`self.itsTrigger?`))
    (`SceneComponent.SetHiddenInGame` (`self.StaticMeshComponent`) _inverted false)
    (set `self.isWorking?` _inverted)
    (set `self.itsOccupied?` false)
    (`/Game/BP_Character/BP_Pawn.CHECK_PROCCESS_EVENT` (`self.bpPawn`))))

(event `CAN_INTERACT_EVENT`
  ;[1 1 1] CAN INTERACT?
  (`self.CHANGE_INDEX_PROCESS_EVENT`)
  (bind _bppawn (`self.bpPawn`)
    (:`then`
      (bind _output_get (set `self.CanInteract?` (== (`/Game/BP_Character/BP_Pawn.index` _bppawn) (`self.process_index`))))
      (if _output_get
        (if (`self.itsTrigger?`)
          (`SceneComponent.SetHiddenInGame` (`self.StaticMeshComponent`) false false))
        (elif (`self.itsTrigger?`)
          (`SceneComponent.SetHiddenInGame` (`self.StaticMeshComponent`) true false))))
    (:`else`)))

(event `CHANGE_INDEX_PROCESS_EVENT`
  (bind _process_index_change (`self.process_index_change`))
  (bind _index (`/Game/BP_Character/BP_Pawn.index` (`self.bpPawn`)))
  ;[1 1 1] CHANGE INDEX PROCESS
  (if (and (> _process_index_change 0) (== _process_index_change _index))
    (set `self.process_index` _index)
    (if (`self.itsTrigger?`)
      (set `self.inverted` (`self.set_inverted_to`))
      (set `self.isWorking?` false)
      (elif (`self.functionality`)
        (set `self.functionality` (not (`self.set_inverted_to`)))))))

(fn `UserConstructionScript`
  (`parent.UserConstructionScript`))