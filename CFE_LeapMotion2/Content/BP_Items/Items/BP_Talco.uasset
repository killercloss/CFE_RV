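; BP_Talco is a talc item that receives dielectric gloves (BP_GuantesDielectricos) when they overlap its static mesh component.
; On overlap, it stores itself in the gloves' BpMiscellaneous reference, snaps them to the mesh while keeping world scale, and calls their CHECKEVENT.
; An ItsOccupied flag then blocks further attachments, and nothing in this Blueprint clears it.
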(event `self.StaticMeshComponent.OnComponentBeginOverlap`
  (params (OverlappedComponent :type "PrimitiveComponent Object Reference") (OtherActor :type "Actor Object Reference") (OtherComp :type "PrimitiveComponent Object Reference") (OtherBodyIndex :type Integer) (bFromSweep :type Boolean) (SweepResult :type "HitResult Structure (by ref)"))
  (if (not (`self.ItsOccupied?`))
    (bind _asbp_guantes_dielectricos (cast `/Game/BP_Items/Items/BP_GuantesDielectricos` OtherActor))
    (set `/Game/BP_Items/Items/BP_Miscelaneus.bpMiscellaneous` self _asbp_guantes_dielectricos)
    (`self.K2_AttachToComponent` _asbp_guantes_dielectricos (`self.StaticMesh`) "None" "SnapToTarget" "SnapToTarget" "KeepWorld" true)
    (`/Game/BP_Items/Items/BP_GuantesDielectricos.CHECK_EVENT` _asbp_guantes_dielectricos)
    (set `self.ItsOccupied?` true)))

(fn `UserConstructionScript`
  (`parent.UserConstructionScript`))