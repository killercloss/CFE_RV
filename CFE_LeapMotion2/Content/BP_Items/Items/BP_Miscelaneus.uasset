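; BP_Miscelaneus is a miscellaneous item that can be picked up and dropped.
; On begin play it caches the player pawn and sets whether it can be interacted with by comparing the pawn's Index to its own ProcessIndex.
; Pickup attaches it to the given hand's ObjectSocket, keeping world transform, and frees the linked BpMiscellaneous by clearing its occupied flag and the reference.
; Drop detaches the static mesh in place.
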(event `self.ReceiveBeginPlay`
  (bind _asbp_pawn (cast `/Game/BP_Character/BP_Pawn` (`GameplayStatics.GetPlayerPawn` 0)))
  (set `self.bpPawn` _asbp_pawn)
  (`self.CAN_INTERACT_EVENT`))

(event `/Game/BP_Items/BP_ItemInterface.ItemPickUp`
  (params (HandToAttach :type "SkeletalMeshComponent Object Reference"))
  (`self.K2_AttachToComponent` self HandToAttach "ObjectSocket" "KeepWorld" "KeepWorld" "KeepWorld" true)
  (bind _bpmiscellaneous (`self.bpMiscellaneous`)
    (:`then`
      (set `/Game/BP_Items/Items/BP_Miscelaneus.ItsOccupied?` false _bpmiscellaneous)
      (set `self.bpMiscellaneous` null))
    (:`else`)))

(event `/Game/BP_Items/BP_ItemInterface.ItemDrop`
  (`SceneComponent.K2_DetachFromComponent` (`self.StaticMeshComponent`) "KeepWorld" "KeepWorld" "KeepWorld" true))

(event `CAN_INTERACT_EVENT`
  (bind _bppawn (`self.bpPawn`)
    (:`then`
      (set `self.CanInteract?` (== (`/Game/BP_Character/BP_Pawn.index` _bppawn) (`self.processIndex`))))
    (:`else`)))

(fn `UserConstructionScript`
  (`parent.UserConstructionScript`))