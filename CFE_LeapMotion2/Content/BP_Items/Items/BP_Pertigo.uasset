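; BP_Pertigo is a holdable item that acts as a tool, with a Box that other items attach to.
; Pickup and drop events attach it to the hand's ObjectSocket and detach it, keeping world transform.
; While unoccupied, overlapping items register it as their tool, and interactable, non-trigger items of listed classes snap onto the Box.
; A detach event clears the Occupied flag, which this graph never sets true.
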(event `/Game/BP_Items/BP_ItemInterface.ItemPickUp`
  (params (HandToAttach :type "SkeletalMeshComponent Object Reference"))
  (`self.K2_AttachToComponent` self HandToAttach "ObjectSocket" "KeepWorld" "KeepWorld" "KeepWorld" true))

(event `/Game/BP_Items/BP_ItemInterface.ItemDrop`
  (`SceneComponent.K2_DetachFromComponent` (`self.StaticMeshComponent`) "KeepWorld" "KeepWorld" "KeepWorld" true))

(event `self.Box.OnComponentBeginOverlap`
  (params (OverlappedComponent :type "PrimitiveComponent Object Reference") (OtherActor :type "Actor Object Reference") (OtherComp :type "PrimitiveComponent Object Reference") (OtherBodyIndex :type Integer) (bFromSweep :type Boolean) (SweepResult :type "HitResult Structure (by ref)"))
  (if (not (`self.Occupied?`))
    (bind _asbp_item_class (cast `/Game/BP_Items/Items/BP_ItemClass` OtherActor))
    (set `/Game/BP_Items/Items/BP_ItemClass.bpToolClass` self _asbp_item_class)
    (if (and (`/Game/BP_Items/Items/BP_Base.CanInteract?` _asbp_item_class) (not (`/Game/BP_Items/Items/BP_ItemClass.itsTrigger?` _asbp_item_class)) (>= (`KismetArrayLibrary.Array_Find` (`self.Classes`) (`GameplayStatics.GetObjectClass` _asbp_item_class)) 0))
      (`self.K2_AttachToComponent` _asbp_item_class (`self.Box`) "None" "SnapToTarget" "SnapToTarget" "KeepWorld" true))))

(event `DETTACH_EVENT`
  (set `self.Occupied?` false))

(fn `UserConstructionScript`
  (`parent.UserConstructionScript`))