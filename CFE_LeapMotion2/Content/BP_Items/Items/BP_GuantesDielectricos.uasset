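; Dielectric gloves item that the player inspects, where each instance is either working or faulty.
; Checking a working pair marks it checked, while a faulty one flashes a particle effect for one second.
; A scan of same-class actors stops at the first unchecked working pair, flagging any checked one before it.
; That flag, intended as an all-checked test, sets the pawn's index and triggers its interaction check.
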(event `CHECK_EVENT`
  (bind _particlesystem (`self.ParticleSystem`))
  (if (`self.isWorking?`)
    (set `self.checked` true)
    (`self.CHECK_EVERY_GLOVE`)
    (else
      (`ActorComponent.Activate` _particlesystem false)
      (`KismetSystemLibrary.Delay` 1.0)
      (`ActorComponent.Deactivate` _particlesystem))))

(event `CHECK_EVERY_GLOVE`
  (bind _bppawn (`self.bpPawn`))
  (bind _outactors (`GameplayStatics.GetAllActorsOfClass` (`GameplayStatics.GetObjectClass` self)))
  (for _array_element _outactors
    (if (`/Game/BP_Items/Items/BP_GuantesDielectricos.isWorking?` _array_element)
      (if (`/Game/BP_Items/Items/BP_GuantesDielectricos.checked` _array_element)
        (set `self.mustAdd?` true)
        (else
          (break)))))
  (if (`self.mustAdd?`)
    (set `/Game/BP_Character/BP_Pawn.index` (`self.indexToIncrement`) _bppawn)
    (`/Game/BP_Character/BP_Pawn.CHECK_CAN_INTERACT_EVENT` _bppawn)))

(fn `UserConstructionScript`
  (`parent.UserConstructionScript`))