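; BP_Pawn is a pawn that creates the BP_WManiobras widget on BeginPlay and tracks progress through a series of percentage values.
; AddEvt raises the current Percent entry and advances Index once that entry reaches 100 or more, without capping it.
; SubEvt lowers the current entry, flooring it at zero, and never moves Index back.
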(event `self.ReceiveBeginPlay`
  (bind _returnvalue (`|CreateWidget` "/Game/BP_Character/BP_WManiobras.BP_WManiobras_C" (`GameplayStatics.GetPlayerController` 0)))
  (`UserWidget.AddToViewport` _returnvalue 0))

(event `AddEvt`
  (params (Amount :type Integer))
  (bind _percent (`self.Percent`))
  (bind _index (`self.index`))
  (bind _output (`|GetArrayItem` _percent _index))
  (`KismetArrayLibrary.Array_Set` _percent _index (+ Amount _output))
  (if (>= _output 100)
    (set `self.index` (+ (`self.index`) 1))))

(event `SubEvt`
  (params (Amount :type Integer))
  (bind _percent (`self.Percent`))
  (bind _index (`self.index`))
  (bind _returnvalue (- (`|GetArrayItem` _percent _index) Amount))
  (if (< _returnvalue 0)
    (`KismetArrayLibrary.Array_Set` _percent _index)
    (else
      (`KismetArrayLibrary.Array_Set` _percent _index _returnvalue))))

(fn `UserConstructionScript`)